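; BP_DyeBucket is a dye bucket that gives an overlapping pickup the bucket's color.
; On Interact, it takes the first BP_PickupBase overlapping its BoxCollision and sets that pickup's CurrentColor to BucketColor.
; The construction script creates a dynamic material on the static mesh and sets its BaseColor parameter to BucketColor, so each bucket shows the dye it applies.
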(event EventInteract
  (params (Instigator :type BP%20First%20Person%20Character%20Object%20Reference%20%28by%20ref%29))
  (bind _boxcollision (Variables|Default|GetBoxCollision))
  (bind _overlappingactors (Collision|GetOverlappingActors _boxcollision "/Game/CaseDir/Blueprints/BP_PickupBase.BP_PickupBase_C" :!class /Script/Engine.PrimitiveComponent))
  (bind _output (Utilities|Array|Get(acopy) _overlappingactors))
  (Utilities|IsValid _output
    (:Is%20Valid
      (bind _asbp_pickup_base (Utilities|Casting|CastToBP_PickupBase _output))
      (Variables|/Game/CaseDir/Blueprints/BP_PickupBase.BP_PickupBase_C|SetCurrentColor _asbp_pickup_base (Variables|Default|GetBucketColor)))))

(fn ConstructionScript
  (bind _returnvalue (Rendering|Material|CreateDynamicMaterialInstance (Variables|Default|GetStaticMesh) 0 0 "None" :!class /Script/Engine.PrimitiveComponent))
  (Rendering|Material|SetVectorParameterValue _returnvalue "BaseColor" (Variables|Default|GetBucketColor) :!class /Script/Engine.MaterialInstanceDynamic))
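; Delivery zone actor that displays the current order as a colored shape hologram and pays out for pickups dropped into it.
; It binds to the game state's order update; the hologram takes the order's mesh and dynamic material color, hiding while waiting.
; On box overlap, the server pays full reward with a multicast cash sound for matching shape and color, half for shape only, nothing otherwise.
; Every delivery destroys the pickup and requests a new order.
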(event OnComponentBeginOverlap(Box)
  (params (OverlappedComponent :type Primitive%20Component%20Object%20Reference) (OtherActor :type Actor%20Object%20Reference) (OtherComp :type Primitive%20Component%20Object%20Reference) (OtherBodyIndex :type Integer) (bFromSweep :type Boolean) (SweepResult :type Hit%20Result%20Structure%20%28by%20ref%29))
  (bind _as_bp_carpenter_game_state (Variables|Default|GetAs%20BP%20Carpenter%20Game%20State))
  (bind _as_bp_carpenter_game_state_2 (Variables|Default|GetAs%20BP%20Carpenter%20Game%20State))
  (bind _as_bp_carpenter_game_state_3 (Variables|Default|GetAs%20BP%20Carpenter%20Game%20State))
  (bind _as_bp_carpenter_game_state_4 (Variables|Default|GetAs%20BP%20Carpenter%20Game%20State))
  (bind _asbp_pickup_base (Utilities|Casting|CastToBP_PickupBase OtherActor))
  (Variables|Default|SetAs%20BP%20Pickup%20Base _asbp_pickup_base)
  (Networking|SwitchHasAuthority
    (:Authority
      (if (Utilities|Enum|Equal(Enum) (Variables|/Game/CaseDir/Blueprints/BP_CarpenterGameState.BP_CarpenterGameState_C|GetOrder_ObjectType _as_bp_carpenter_game_state) (Variables|/Game/CaseDir/Blueprints/BP_PickupBase.BP_PickupBase_C|GetObjectType (Variables|Default|GetAs%20BP%20Pickup%20Base)))
        (if (Class|KismetMathLibrary|LinearColorIsNearEqual (Variables|/Game/CaseDir/Blueprints/BP_CarpenterGameState.BP_CarpenterGameState_C|GetOrder_Color _as_bp_carpenter_game_state) (Variables|/Game/CaseDir/Blueprints/BP_PickupBase.BP_PickupBase_C|GetCurrentColor (Variables|Default|GetAs%20BP%20Pickup%20Base)) 0.01)
          (Variables|/Game/CaseDir/Blueprints/BP_CarpenterGameState.BP_CarpenterGameState_C|SetBudget _as_bp_carpenter_game_state_2 (+ (Variables|/Game/CaseDir/Blueprints/BP_CarpenterGameState.BP_CarpenterGameState_C|GetOrder_Reward _as_bp_carpenter_game_state_4) (Variables|/Game/CaseDir/Blueprints/BP_CarpenterGameState.BP_CarpenterGameState_C|GetBudget _as_bp_carpenter_game_state_4)))
          (CallFunction|MulticastDeliveryEffect (Transformation|GetActorLocation (Variables|Default|GetAs%20BP%20Pickup%20Base)))
          (else
            (Variables|/Game/CaseDir/Blueprints/BP_CarpenterGameState.BP_CarpenterGameState_C|SetBudget _as_bp_carpenter_game_state_4 (+ (/ (Variables|/Game/CaseDir/Blueprints/BP_CarpenterGameState.BP_CarpenterGameState_C|GetOrder_Reward _as_bp_carpenter_game_state_3) 2) (Variables|/Game/CaseDir/Blueprints/BP_CarpenterGameState.BP_CarpenterGameState_C|GetBudget _as_bp_carpenter_game_state_3)))))
        (Actor|DestroyActor (Variables|Default|GetAs%20BP%20Pickup%20Base))
        (Default|ServerCreateNewOrder _as_bp_carpenter_game_state_2)
        (else
          (Actor|DestroyActor (Variables|Default|GetAs%20BP%20Pickup%20Base))
          (Default|ServerCreateNewOrder _as_bp_carpenter_game_state_3))))))

(event Custom|Multicast_DeliveryEffect
  (params (Location :type Vector))
  (Audio|PlaySoundatLocation "/Game/CaseDir/Sfx/sfx_cash.sfx_cash" Location "0, 0, 0" 1.0 1.0 0.0 0 0 0 0))

(event Custom|UpdateHologram
  (params (NewObject :type E_ObjectTypes%20Enum :default "NewEnumerator0") (NewColor :type Linear%20Color%20Structure))
  (bind _hologrammesh (Variables|Default|GetHologramMesh))
  (bind _hologrammesh_2 (Variables|Default|GetHologramMesh))
  (if (Utilities|Enum|Equal(Enum) NewObject "NewEnumerator4")
    (Rendering|SetVisibility _hologrammesh false false)
    (else
      (Rendering|SetVisibility _hologrammesh true false)
      (switch Utilities|FlowControl|Switch|SwitchonE_ObjectTypes (Variables|/Game/CaseDir/Blueprints/BP_CarpenterGameState.BP_CarpenterGameState_C|GetOrder_ObjectType (Variables|Default|GetAs%20BP%20Carpenter%20Game%20State))
        (:NewEnumerator0
          (Components|StaticMesh|SetStaticMesh _hologrammesh_2 "/Game/LevelPrototyping/Meshes/SM_ChamferCube.SM_ChamferCube"))
        (:NewEnumerator1
          (Components|StaticMesh|SetStaticMesh _hologrammesh_2 "/Game/LevelPrototyping/Meshes/SM_Cylinder.SM_Cylinder"))
        (:NewEnumerator2
          (Components|StaticMesh|SetStaticMesh _hologrammesh_2 "/Game/AssetSource/SM_Sphere.SM_Sphere")))
      (bind _returnvalue (Rendering|Material|CreateDynamicMaterialInstance (Variables|Default|GetHologramMesh) 0 0 "None" :!class /Script/Engine.PrimitiveComponent))
      (Rendering|Material|SetVectorParameterValue _returnvalue "Color" NewColor :!class /Script/Engine.MaterialInstanceDynamic))))

(event EventBeginPlay
  (bind _asbp_carpenter_game_state (Utilities|Casting|CastToBP_CarpenterGameState (Game|GetGameState)))
  (bind _output_get (Variables|Default|SetAs%20BP%20Carpenter%20Game%20State _asbp_carpenter_game_state))
  (EventDispatchers|BindEventtoEDOrderUpdate _output_get (EventDispatchers|CreateEvent :!event Custom|UpdateHologram))
  (Components|Movement|SetUpdatedComponent (Variables|Default|GetRotatingMovement) (Variables|Default|GetBox)))

(fn ConstructionScript)
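; BP_PickupBase is a pickup actor that a player holds in the right hand, with replicated holder and color state.
; Interact sets HoldingPlayer, whose RepNotify disables physics and collision, snaps the pickup to the HandGrip_R socket and sets the player's HeldObject.
; When the holder is invalid, the same RepNotify detaches it and restores physics and collision.
; The CurrentColor RepNotify applies the color through a dynamic material instance.
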(event EventInteract
  (params (Instigator :type BP%20First%20Person%20Character%20Object%20Reference%20%28by%20ref%29))
  (Variables|Default|SetHoldingPlayer Instigator))

(fn ConstructionScript)

(fn OnRepHoldingPlayer
  (bind _staticmesh (Variables|Default|GetStaticMesh))
  (bind _holdingplayer (Variables|Default|GetHoldingPlayer))
  (Utilities|IsValid _holdingplayer
    (:Is%20Valid
      (Physics|SetSimulatePhysics _staticmesh false)
      (Collision|SetCollisionEnabled _staticmesh "NoCollision")
      (Transformation|AttachComponentToComponent (Variables|/Script/Engine.Character|GetMesh _holdingplayer) "HandGrip_R" "SnapToTarget" "SnapToTarget" "KeepWorld" true)
      (Variables|/Game/FirstPerson/Blueprints/BP_FirstPersonCharacter.BP_FirstPersonCharacter_C|SetHeldObject _holdingplayer self))
    (:Is%20Not%20Valid
      (Transformation|DetachFromActor "KeepWorld" "KeepWorld" "KeepWorld")
      (Collision|SetCollisionEnabled (Variables|Default|GetStaticMesh) "QueryAndPhysics")
      (Physics|SetSimulatePhysics (Variables|Default|GetStaticMesh) true))))

(fn OnRepCurrentColor
  (bind _returnvalue (Rendering|Material|CreateDynamicMaterialInstance (Variables|Default|GetStaticMesh) 0 0 "None" :!class /Script/Engine.PrimitiveComponent))
  (Rendering|Material|SetVectorParameterValue _returnvalue "ObjectColor" (Variables|Default|GetCurrentColor) :!class /Script/Engine.MaterialInstanceDynamic))